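; BP_Tile is a terrain segment for an infinite terrain game, exposing an arrow transform as the attach location.
; When the player enters the LockingVolume, it unlocks its barrier (no collision, green material) and asks the InfiniteTerrainGameMode to spawn the next tile.
; Leaving that volume locks the barrier again (collision, red material).
; The player entering the LifeVolume destroys the tile.
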(event `self.ReceiveBeginPlay`)

(event `self.LockingVolume.OnComponentBeginOverlap`
  (params (OverlappedComponent :type "PrimitiveComponent Object Reference") (OtherActor :type "Actor Object Reference") (OtherComp :type "PrimitiveComponent Object Reference") (OtherBodyIndex :type Integer) (bFromSweep :type Boolean) (SweepResult :type "HitResult Structure (by ref)"))
  (`self.is Player Actor` OtherActor)
  (`self.Unlock`)
  (bind _asinfinite_terrain_game_mode (cast `/Game/Dynamic/InfiniteTerrainGameMode` (`GameplayStatics.GetGameMode`)))
  (`/Game/Dynamic/InfiniteTerrainGameMode.Spawn Next Tile` _asinfinite_terrain_game_mode))

(event `self.LockingVolume.OnComponentEndOverlap`
  (params (OverlappedComponent :type "PrimitiveComponent Object Reference") (OtherActor :type "Actor Object Reference") (OtherComp :type "PrimitiveComponent Object Reference") (OtherBodyIndex :type Integer))
  (`self.is Player Actor` OtherActor)
  (`self.Lock`))

(event `self.LifeVolume.OnComponentBeginOverlap`
  (params (OverlappedComponent :type "PrimitiveComponent Object Reference") (OtherActor :type "Actor Object Reference") (OtherComp :type "PrimitiveComponent Object Reference") (OtherBodyIndex :type Integer) (bFromSweep :type Boolean) (SweepResult :type "HitResult Structure (by ref)"))
  (`self.is Player Actor` OtherActor)
  (`self.K2_DestroyActor`))

(fn `Get Attach Location`
  (returns (`Attach Transform` :type "Transform Structure"))
  (return (`SceneComponent.K2_GetComponentToWorld` (`self.Arrow`))))

(fn `Lock`
  (`PrimitiveComponent.SetCollisionEnabled` (`self.StaticMeshComponent_Barrier`) "QueryAndPhysics")
  (`PrimitiveComponent.SetMaterial` (`self.StaticMeshComponent_Barrier`) 0 "/Game/Static/Geometry/Meshes/BarrierMaterial_Inst_Red.BarrierMaterial_Inst_Red"))

(fn `Unlock`
  (`PrimitiveComponent.SetCollisionEnabled` (`self.StaticMeshComponent_Barrier`) "NoCollision")
  (`PrimitiveComponent.SetMaterial` (`self.StaticMeshComponent_Barrier`) 0 "/Game/Static/Geometry/Meshes/BarrierMaterial_Inst_Green.BarrierMaterial_Inst_Green"))

(fn `UserConstructionScript`)